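; Order manager for the delivery rover game: generates, tracks and resolves delivery orders and feeds the HUD.
; A looping timer adds randomized orders of four types, routed between cached BP_OrderLocationMarker actors, up to a cap.
; Accepting an order starts a DeliveryState flow that spawns pickup, then delivery points, advanced by TryInteract and failed by timeout or cargo collision damage.
; Tick pushes state, distance, battery, cargo and charging prompts to the player controller's HUD widget.
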(event `self.ReceiveBeginPlay`
  (`self.CacheLocationMarkers`)
  (`self.GenerateRandomOrder`)
  (`KismetSystemLibrary.K2_SetTimer` null "GenerateRandomOrder" (`self.OrderSpawnInterval`) true))

(event `self.ReceiveTick`
  (params (DeltaSeconds :type "Float (single-precision)"))
  (bind _deliverystate (`self.DeliveryState`))
  (`|ExecutionSequence`
    (:`then_0`
      (`self.UpdateHUD`))
    (:`then_1`
      (if (`self.bHasActiveOrder`)
        (if (or (`|EnumEquality` _deliverystate "NewEnumerator1") (`|EnumEquality` _deliverystate "NewEnumerator2"))
          (set `self.RemainingTime` (`KismetMathLibrary.FClamp` (- (`self.RemainingTime`) DeltaSeconds) 0.0 9999.0))
          (if (<= (`self.RemainingTime`) 0.0)
            (set `self.DeliveryState` "NewEnumerator4")
            (set `self.bHasActiveOrder` false)
            (set `self.bRoverAtPickup` false)
            (set `self.bRoverAtDelivery` false)
            (`self.ClearActiveOrderPoints`)))))))

(fn `AcceptOrderByID`
  (params (OrderID :type Integer))
  (if (`self.bHasActiveOrder`)
    (`KismetSystemLibrary.PrintString` "Уже есть активный заказ. Сначала завершите доставку.")
    (else
      (set `self.CargoPercent` 1.0)
      (set `self.CollisionCount` 0)
      (for (_array_element _array_index) (`self.AvailableOrders`)
        (if (== OrderID (`.OrderID_2_41312DDB4DBF8C64495B019AD6B0CCE1` (break `/Game/DeliveryRover/Blueprints/Gameplay/ST_DeliveryOrder` _array_element)))
          (set `self.ActiveOrder` _array_element)
          (set `self.bHasActiveOrder` true)
          (set `self.DeliveryState` "NewEnumerator1")
          (set `self.bRoverAtPickup` false)
          (set `self.bRoverAtDelivery` false)
          (set `self.CargoPercent` 1.0)
          (set `self.RemainingTime` (`.TimeLimit_19_03363D6B4C855C0CE6DEAB808B3956C8` (break `/Game/DeliveryRover/Blueprints/Gameplay/ST_DeliveryOrder` (`self.ActiveOrder`))))
          (`KismetArrayLibrary.Array_Remove` (`self.AvailableOrders`) _array_index)
          (break)))
      (`KismetSystemLibrary.PrintString` "Calling SpawnActivePickupPoint")
      (`self.SpawnActivePickupPoint`)
      (`self.OnOrdersUpdated`)
      (`KismetSystemLibrary.PrintString` "Заказ принят. Езжайте к точке забора"))))

(fn `CacheLocationMarkers`
  (bind _pickupmarkers (`self.PickupMarkers`))
  (bind _deliverymarkers (`self.DeliveryMarkers`))
  (`KismetArrayLibrary.Array_Clear` (`self.LocationMarkers`))
  (`KismetArrayLibrary.Array_Clear` (`self.PickupMarkers`))
  (`KismetArrayLibrary.Array_Clear` (`self.DeliveryMarkers`))
  (bind _outactors (`GameplayStatics.GetAllActorsOfClass` "/Game/DeliveryRover/Blueprints/Gameplay/OrderLocations/BP_OrderLocationMarker.BP_OrderLocationMarker_C"))
  (for _array_element _outactors
    (bind _asbp_order_location_marker (cast `/Game/DeliveryRover/Blueprints/Gameplay/OrderLocations/BP_OrderLocationMarker` _array_element))
    (if (`/Game/DeliveryRover/Blueprints/Gameplay/OrderLocations/BP_OrderLocationMarker.bIsAvailable` _asbp_order_location_marker)
      (`KismetArrayLibrary.Array_Add` (`self.LocationMarkers`) _array_element)
      (switch `/Game/DeliveryRover/Blueprints/Gameplay/E_OrderLocationType` (`/Game/DeliveryRover/Blueprints/Gameplay/OrderLocations/BP_OrderLocationMarker.LocationType` _asbp_order_location_marker)
        (:`NewEnumerator0`
          (`KismetArrayLibrary.Array_Add` _pickupmarkers _array_element))
        (:`NewEnumerator1`
          (`KismetArrayLibrary.Array_Add` _deliverymarkers _array_element))
        (:`NewEnumerator2`
          (`|ExecutionSequence`
            (:`then_0`
              (`KismetArrayLibrary.Array_Add` _deliverymarkers _array_element))
            (:`then_1`
              (`KismetArrayLibrary.Array_Add` _pickupmarkers _array_element))))))))

(fn `ClearActiveOrderPoints`
  (bind _activepickuppointref (`self.ActivePickupPointRef`))
  (bind _activedeliverypointref (`self.ActiveDeliveryPointRef`))
  (`|ExecutionSequence`
    (:`then_0`
      (`/Engine/EditorBlueprintResources/StandardMacros.IsValid` _activepickuppointref
        (:`Is Valid`
          (`self.K2_DestroyActor` _activepickuppointref)
          (set `self.ActivePickupPointRef` null))))
    (:`then_1`
      (`/Engine/EditorBlueprintResources/StandardMacros.IsValid` _activedeliverypointref
        (:`Is Valid`
          (`self.K2_DestroyActor` _activedeliverypointref)
          (set `self.ActiveDeliveryPointRef` null))))))

(fn `FailCurrentDelivery`
  (params (FailReason :type Text))
  (set `self.DeliveryState` "NewEnumerator4")
  (set `self.bHasActiveOrder` false)
  (set `self.bRoverAtPickup` false)
  (set `self.bRoverAtDelivery` false)
  (`self.ClearActiveOrderPoints`)
  (`self.OnOrdersUpdated`))

(fn `GenerateRandomOrder`
  (locals (SelectedPickupMarker :type "/Game/DeliveryRover/Blueprints/Gameplay/OrderLocations/BP_OrderLocationMarker Object Reference") (SelectedDeliveryMarker :type "/Game/DeliveryRover/Blueprints/Gameplay/OrderLocations/BP_OrderLocationMarker Object Reference"))
  (bind _selectedpickupmarker (`local.SelectedPickupMarker`))
  (bind _selecteddeliverymarker (`local.SelectedDeliveryMarker`))
  (bind _availableorders (`self.AvailableOrders`))
  (bind _returnvalue (`self.GetTransform` _selecteddeliverymarker))
  (bind _returnvalue_2 (`self.GetTransform` _selectedpickupmarker))
  (bind _locationname (`/Game/DeliveryRover/Blueprints/Gameplay/OrderLocations/BP_OrderLocationMarker.LocationName` _selectedpickupmarker))
  (bind _locationname_2 (`/Game/DeliveryRover/Blueprints/Gameplay/OrderLocations/BP_OrderLocationMarker.LocationName` _selecteddeliverymarker))
  (if (< (`KismetArrayLibrary.Array_Length` (`self.AvailableOrders`)) (`self.MaxAvailableOrders`)) :!label _label
    (bind _output_get (set `self.NextOrderID` (+ (`self.NextOrderID`) 1)))
    (if (> (`KismetArrayLibrary.Array_Length` (`self.PickupMarkers`)) 0)
      (if (> (`KismetArrayLibrary.Array_Length` (`self.DeliveryMarkers`)) 0)
        (`|ExecutionSequence`
          (:`then_0`
            (bind _output_get_2 (set `local.SelectedPickupMarker` (`|GetArrayItem` (`self.PickupMarkers`) (`KismetMathLibrary.RandomIntegerInRange` 0 (- (`KismetArrayLibrary.Array_Length` (`self.PickupMarkers`)) 1))))))
          (:`then_1`
            (bind _output_get_3 (set `local.SelectedDeliveryMarker` (`|GetArrayItem` (`self.DeliveryMarkers`) (`KismetMathLibrary.RandomIntegerInRange` 0 (- (`KismetArrayLibrary.Array_Length` (`self.DeliveryMarkers`)) 1))))))
          (:`then_2`
            (if (== _output_get_2 _output_get_3)
              (goto _label)
              (else
                (switch `int` (`KismetMathLibrary.RandomIntegerInRange` 0 3)
                  (:`0`
                    (`KismetArrayLibrary.Array_Add` _availableorders (make `/Game/DeliveryRover/Blueprints/Gameplay/ST_DeliveryOrder` _output_get "Обычная доставка" "NewEnumerator0" (`KismetMathLibrary.RandomIntegerInRange` 80 140) (`KismetMathLibrary.Conv_IntToDouble` (`KismetMathLibrary.RandomIntegerInRange` 180 240)) (`KismetMathLibrary.RandomIntegerInRange` 1 2) "300–500 м" 1.0 _returnvalue_2 _returnvalue _locationname _locationname_2))
                    (`KismetSystemLibrary.PrintString` "Order added Normal"))
                  (:`1`
                    (`KismetArrayLibrary.Array_Add` _availableorders (make `/Game/DeliveryRover/Blueprints/Gameplay/ST_DeliveryOrder` _output_get "Срочная доставка" "NewEnumerator1" (`KismetMathLibrary.RandomIntegerInRange` 180 250) (`KismetMathLibrary.Conv_IntToDouble` (`KismetMathLibrary.RandomIntegerInRange` 90 150)) (`KismetMathLibrary.RandomIntegerInRange` 3 4) "400–700 м" 1.0 _returnvalue_2 _returnvalue _locationname _locationname_2))
                    (`KismetSystemLibrary.PrintString` "Order added Urgent"))
                  (:`2`
                    (`KismetArrayLibrary.Array_Add` _availableorders (make `/Game/DeliveryRover/Blueprints/Gameplay/ST_DeliveryOrder` _output_get "Хрупкая посылка" "NewEnumerator2" (`KismetMathLibrary.RandomIntegerInRange` 200 300) (`KismetMathLibrary.Conv_IntToDouble` (`KismetMathLibrary.RandomIntegerInRange` 180 260)) (`KismetMathLibrary.RandomIntegerInRange` 4 5) "350–650 м" 2.0 _returnvalue_2 _returnvalue _locationname _locationname_2))
                    (`KismetSystemLibrary.PrintString` "Order added Fragile"))
                  (:`3`
                    (`KismetArrayLibrary.Array_Add` _availableorders (make `/Game/DeliveryRover/Blueprints/Gameplay/ST_DeliveryOrder` _output_get "Дальняя доставка" "NewEnumerator3" (`KismetMathLibrary.RandomIntegerInRange` 220 350) (`KismetMathLibrary.Conv_IntToDouble` (`KismetMathLibrary.RandomIntegerInRange` 240 360)) (`KismetMathLibrary.RandomIntegerInRange` 3 5) "700–1000 м" 1.0 _returnvalue_2 _returnvalue _locationname _locationname_2))
                    (`KismetSystemLibrary.PrintString` "Order added LongDistance")))
                (`self.OnOrdersUpdated`)))))))))

(fn `GetDistanceTextToCurrentTarget`
  (returns (DistanceText :type Text))
  (bind _activepickuppointref (`self.ActivePickupPointRef`))
  (bind _activedeliverypointref (`self.ActiveDeliveryPointRef`))
  (switch `/Game/DeliveryRover/Blueprints/Gameplay/E_DeliveryState` (`self.DeliveryState`)
    (:`NewEnumerator0`
      _)
    (:`NewEnumerator1`
      (`/Engine/EditorBlueprintResources/StandardMacros.IsValid` _activepickuppointref
        (:`Is Valid`
          (return (`|FormatText` "До точки забора: {Distance} м" (`KismetMathLibrary.Round` (/ (`KismetMathLibrary.Vector_Distance` (`self.K2_GetActorLocation` (`GameplayStatics.GetPlayerPawn` 0)) (`self.K2_GetActorLocation` _activepickuppointref)) 100.0)))))
        (:`Is Not Valid`
          _)))
    (:`NewEnumerator2`
      (`/Engine/EditorBlueprintResources/StandardMacros.IsValid` _activedeliverypointref
        (:`Is Valid`
          (return (`|FormatText` "До точки доставки: {Distance} м" (`KismetMathLibrary.Round` (/ (`KismetMathLibrary.Vector_Distance` (`self.K2_GetActorLocation` (`GameplayStatics.GetPlayerPawn` 0)) (`self.K2_GetActorLocation` _activedeliverypointref)) 100.0)))))
        (:`Is Not Valid`
          _)))
    (:`NewEnumerator3`
      _)
    (:`NewEnumerator4`
      _))
  (return "До цели: —"))

(fn `RegisterCollisionDamage`
  (params (BaseDamage :type "Float (double-precision)" :default 0.05))
  (bind _returnvalue (`KismetSystemLibrary.GetGameTimeInSeconds`))
  (if (>= (- _returnvalue (`self.LastCollisionDamageTime`)) (`self.CollisionDamageCooldown`))
    (set `self.LastCollisionDamageTime` _returnvalue)
    (if (`self.bHasActiveOrder`)
      (if (`|EnumEquality` (`self.DeliveryState`) "NewEnumerator2")
        (set `self.CollisionCount` (+ (`self.CollisionCount`) 1))
        (bind _output_get (set `self.CargoPercent` (`KismetMathLibrary.FClamp` (- (`self.CargoPercent`) (* BaseDamage (`.CargoDamageMultiplier_17_84AC50554660C82D4B29358A0E951E1C` (break `/Game/DeliveryRover/Blueprints/Gameplay/ST_DeliveryOrder` (`self.ActiveOrder`))))))))
        (if (<= _output_get 0.0)
          (`self.FailCurrentDelivery` "Посылка полностью повреждена"))))))

(fn `SetRoverAtDelivery`
  (set `self.bRoverAtDelivery` true))

(fn `SetRoverAtPickup`
  (set `self.bRoverAtPickup` true))

(fn `SetRoverLeftDelivery`
  (set `self.bRoverAtDelivery` false))

(fn `SetRoverLeftPickup`
  (set `self.bRoverAtPickup` false))

(fn `SpawnActiveDeliveryPoint`
  (bind _activedeliverypointref (`self.ActiveDeliveryPointRef`))
  (`/Engine/EditorBlueprintResources/StandardMacros.IsValid` _activedeliverypointref
    (:`Is Valid`
      (`self.K2_DestroyActor` _activedeliverypointref))
    (:`Is Not Valid`
      _))
  (bind _returnvalue (`|SpawnActorFromClass` (`self.DeliveryPointClass`) (`.DeliveryTransform_31_5B9E0175497B615173D63E9512129DC3` (break `/Game/DeliveryRover/Blueprints/Gameplay/ST_DeliveryOrder` (`self.ActiveOrder`))) "Undefined" "MultiplyWithRoot" null null))
  (set `self.ActiveDeliveryPointRef` _returnvalue))

(fn `SpawnActivePickupPoint`
  (bind _activepickuppointref (`self.ActivePickupPointRef`))
  (`KismetSystemLibrary.PrintString` "SpawnActivePickupPoint started")
  (`/Engine/EditorBlueprintResources/StandardMacros.IsValid` _activepickuppointref
    (:`Is Valid`
      (`self.K2_DestroyActor` _activepickuppointref))
    (:`Is Not Valid`
      _))
  (bind _returnvalue (`|SpawnActorFromClass` (`self.PickupPointClass`) (`.PickupTransform_30_D8ABD1824F1B3B3ACC7123824D0C818C` (break `/Game/DeliveryRover/Blueprints/Gameplay/ST_DeliveryOrder` (`self.ActiveOrder`))) "Undefined" "MultiplyWithRoot" null null))
  (set `self.ActivePickupPointRef` _returnvalue))

(fn `TryInteract`
  (switch `/Game/DeliveryRover/Blueprints/Gameplay/E_DeliveryState` (`self.DeliveryState`)
    (:`NewEnumerator0`
      (`KismetSystemLibrary.PrintString` "Сначала выберите заказ в приложении"))
    (:`NewEnumerator1`
      (if (`self.bRoverAtPickup`)
        (set `self.DeliveryState` "NewEnumerator2")
        (`self.K2_DestroyActor` (`self.ActivePickupPointRef`))
        (set `self.ActivePickupPointRef` null)
        (set `self.bRoverAtPickup` false)
        (`self.SpawnActiveDeliveryPoint`)
        (`KismetSystemLibrary.PrintString` "Посылка забрана. Езжайте к точке доставки")
        (else
          (`KismetSystemLibrary.PrintString` "Доберитесь до точки забора"))))
    (:`NewEnumerator2`
      (if (`self.bRoverAtDelivery`)
        (set `self.DeliveryState` "NewEnumerator3")
        (set `self.bHasActiveOrder` false)
        (set `self.bRoverAtDelivery` false)
        (`self.ClearActiveOrderPoints`)
        (else
          (`KismetSystemLibrary.PrintString` "Доберитесь до точки доставки"))))
    (:`NewEnumerator3`
      (`KismetSystemLibrary.PrintString` "Доставка уже завершена"))
    (:`NewEnumerator4`
      (`KismetSystemLibrary.PrintString` "Доставка провалена"))))

(fn `UpdateHUD`
  (locals (HUD_ObjectiveText :type Text) (HUD_OrderTitleText :type Text) (HUD_RouteText :type Text) (HUD_TimerText :type Text) (HUD_RewardText :type Text) (HUD_DistanceText :type Text) (HUD_HintText :type Text) (HUD_InteractionPromptText :type Text) (HUD_bShowInteractionPrompt :type Boolean) (HUD_BatteryPercent :type "Float (double-precision)") (HUD_CargoPercent :type "Float (double-precision)") (HUD_BatteryText :type Text) (HUD_CargoText :type Text) (HUD_CollisionsText :type Text))
  (bind _cargopercent (`self.CargoPercent`))
  (bind (_orderid _ordertitle _ordertype _reward _timelimit _difficulty _distancetext _cargodamagemultiplier _pickuptransform _deliverytransform _pickupname _deliveryname) (break `/Game/DeliveryRover/Blueprints/Gameplay/ST_DeliveryOrder` (`self.ActiveOrder`)))
  (bind _asbp_delivery_player_controller (cast `/Game/DeliveryRover/Blueprints/Core/BP_DeliveryPlayerController` (`GameplayStatics.GetPlayerController` 0)))
  (bind _gamehudref (`/Game/DeliveryRover/Blueprints/Core/BP_DeliveryPlayerController.GameHUDRef` _asbp_delivery_player_controller))
  (`/Engine/EditorBlueprintResources/StandardMacros.IsValid` _gamehudref
    (:`Is Valid`
      (`|ExecutionSequence`
        (:`then_0`
          (switch `/Game/DeliveryRover/Blueprints/Gameplay/E_DeliveryState` (`self.DeliveryState`)
            (:`NewEnumerator0`
              (set `local.HUD_ObjectiveText` "Цель: выберите заказ в приложении")
              (set `local.HUD_OrderTitleText` "Заказ: —")
              (set `local.HUD_RouteText` "Маршрут: —")
              (set `local.HUD_TimerText` "Время: —")
              (set `local.HUD_RewardText` "Награда: —")
              (bind _distancetext_2 (`self.GetDistanceTextToCurrentTarget`))
              (set `local.HUD_DistanceText` _distancetext_2)
              (set `local.HUD_HintText` "Tab — открыть приложение заказов")
              (set `local.HUD_InteractionPromptText` "")
              (set `local.HUD_bShowInteractionPrompt` false)
              (bind _asrover_pawn (cast `RoverPawn` (`GameplayStatics.GetPlayerPawn` 0)))
              (bind _returnvalue (`RoverPawn.GetBatteryPercent` _asrover_pawn))
              (set `local.HUD_BatteryPercent` _returnvalue)
              (set `local.HUD_BatteryText` (`|FormatText` "Заряд батареи: {Battery}%" (`KismetMathLibrary.Round` (* _returnvalue 100.0))))
              (set `local.HUD_CargoPercent` 1.0)
              (set `local.HUD_CargoText` "Состояние посылки: —")
              (set `local.HUD_CollisionsText` (`|FormatText` "Столкновения: {Count}" (`self.CollisionCount`))))
            (:`NewEnumerator1`
              (set `local.HUD_ObjectiveText` "Цель: заберите посылку")
              (set `local.HUD_OrderTitleText` (`|FormatText` "Заказ: {Title}" _ordertitle))
              (set `local.HUD_RouteText` (`|FormatText` "Маршрут: {Pickup} → {Delivery}" _pickupname _deliveryname))
              (set `local.HUD_TimerText` (`|FormatText` "Время: {Time} сек." (`KismetMathLibrary.FFloor` (`self.RemainingTime`))))
              (set `local.HUD_RewardText` (`|FormatText` "Награда: {Reward} очков" _reward))
              (bind _distancetext_3 (`self.GetDistanceTextToCurrentTarget`))
              (set `local.HUD_DistanceText` _distancetext_3)
              (set `local.HUD_HintText` "Доберитесь до точки забора")
              (if (`self.bRoverAtPickup`)
                (set `local.HUD_InteractionPromptText` "E — забрать посылку")
                (set `local.HUD_bShowInteractionPrompt` true)
                (else
                  (set `local.HUD_InteractionPromptText` "")
                  (set `local.HUD_bShowInteractionPrompt` false)))
              (bind _asrover_pawn_2 (cast `RoverPawn` (`GameplayStatics.GetPlayerPawn` 0)))
              (bind _returnvalue_2 (`RoverPawn.GetBatteryPercent` _asrover_pawn_2))
              (set `local.HUD_BatteryPercent` _returnvalue_2)
              (set `local.HUD_BatteryText` (`|FormatText` "Заряд батареи: {Battery}%" (`KismetMathLibrary.Round` (* _returnvalue_2 100.0))))
              (set `local.HUD_CargoPercent` 1.0)
              (set `local.HUD_CargoText` "Состояние посылки: —")
              (set `local.HUD_CollisionsText` (`|FormatText` "Столкновения: {Count}" (`self.CollisionCount`))))
            (:`NewEnumerator2`
              (set `local.HUD_ObjectiveText` "Цель: доставьте посылку")
              (set `local.HUD_OrderTitleText` (`|FormatText` "Заказ: {Title}" _ordertitle))
              (set `local.HUD_RouteText` (`|FormatText` "Маршрут: {Pickup} → {Delivery}" _pickupname _deliveryname))
              (set `local.HUD_TimerText` (`|FormatText` "Время: {Time} сек." (`KismetMathLibrary.FFloor` (`self.RemainingTime`))))
              (set `local.HUD_RewardText` (`|FormatText` "Награда: {Reward} очков" _reward))
              (bind _distancetext_4 (`self.GetDistanceTextToCurrentTarget`))
              (set `local.HUD_DistanceText` _distancetext_4)
              (set `local.HUD_HintText` "Доберитесь до точки доставки")
              (if (`self.bRoverAtDelivery`)
                (set `local.HUD_InteractionPromptText` "E — завершить доставку")
                (set `local.HUD_bShowInteractionPrompt` true)
                (else
                  (set `local.HUD_InteractionPromptText` "")
                  (set `local.HUD_bShowInteractionPrompt` false)))
              (bind _asrover_pawn_3 (cast `RoverPawn` (`GameplayStatics.GetPlayerPawn` 0)))
              (bind _returnvalue_3 (`RoverPawn.GetBatteryPercent` _asrover_pawn_3))
              (set `local.HUD_BatteryPercent` _returnvalue_3)
              (set `local.HUD_BatteryText` (`|FormatText` "Заряд батареи: {Battery}%" (`KismetMathLibrary.Round` (* _returnvalue_3 100.0))))
              (set `local.HUD_CargoPercent` _cargopercent)
              (set `local.HUD_CargoText` (`|FormatText` "Состояние посылки: {Cargo}%" (`KismetMathLibrary.Round` (* _cargopercent 100.0))))
              (set `local.HUD_CollisionsText` (`|FormatText` "Столкновения: {Count}" (`self.CollisionCount`))))
            (:`NewEnumerator3`
              (set `local.HUD_ObjectiveText` "Доставка завершена!")
              (set `local.HUD_OrderTitleText` "Заказ выполнен")
              (set `local.HUD_RouteText` "Маршрут завершён")
              (set `local.HUD_TimerText` "Время: завершено")
              (set `local.HUD_RewardText` "Награда начислена")
              (bind _distancetext_5 (`self.GetDistanceTextToCurrentTarget`))
              (set `local.HUD_DistanceText` _distancetext_5)
              (set `local.HUD_HintText` "Tab — выбрать новый заказ")
              (set `local.HUD_InteractionPromptText` "")
              (set `local.HUD_bShowInteractionPrompt` false)
              (bind _asrover_pawn_4 (cast `RoverPawn` (`GameplayStatics.GetPlayerPawn` 0)))
              (bind _returnvalue_4 (`RoverPawn.GetBatteryPercent` _asrover_pawn_4))
              (set `local.HUD_BatteryPercent` _returnvalue_4)
              (set `local.HUD_BatteryText` (`|FormatText` "Заряд батареи: {Battery}%" (`KismetMathLibrary.Round` (* _returnvalue_4 100.0))))
              (set `local.HUD_CargoPercent` 1.0)
              (set `local.HUD_CargoText` "Состояние посылки: —")
              (set `local.HUD_CollisionsText` (`|FormatText` "Столкновения: {Count}" (`self.CollisionCount`))))
            (:`NewEnumerator4`
              (set `local.HUD_ObjectiveText` "Доставка провалена")
              (set `local.HUD_OrderTitleText` "Заказ не выполнен")
              (set `local.HUD_RouteText` "Маршрут отменён")
              (set `local.HUD_TimerText` "Время вышло")
              (set `local.HUD_RewardText` "Награда: 0")
              (bind _distancetext_6 (`self.GetDistanceTextToCurrentTarget`))
              (set `local.HUD_DistanceText` _distancetext_6)
              (set `local.HUD_HintText` "Tab — выбрать новый заказ")
              (set `local.HUD_InteractionPromptText` "")
              (set `local.HUD_bShowInteractionPrompt` false)
              (bind _asrover_pawn_5 (cast `RoverPawn` (`GameplayStatics.GetPlayerPawn` 0)))
              (bind _returnvalue_5 (`RoverPawn.GetBatteryPercent` _asrover_pawn_5))
              (set `local.HUD_BatteryPercent` _returnvalue_5)
              (set `local.HUD_BatteryText` (`|FormatText` "Заряд батареи: {Battery}%" (`KismetMathLibrary.Round` (* _returnvalue_5 100.0))))
              (set `local.HUD_CargoPercent` (`self.CargoPercent`))
              (set `local.HUD_CargoText` "Состояние посылки: -")
              (set `local.HUD_CollisionsText` (`|FormatText` "Столкновения: {Count}" (`self.CollisionCount`))))))
        (:`then_1`
          (bind _asbp_rover_pawn (cast `/Game/DeliveryRover/Blueprints/Rover/BP_RoverPawn` (`GameplayStatics.GetPlayerPawn` 0)))
          (`/Engine/EditorBlueprintResources/StandardMacros.IsValid` (`/Game/DeliveryRover/Blueprints/Rover/BP_RoverPawn.CurrentChargingStation` _asbp_rover_pawn)
            (:`Is Valid`
              (if (`/Game/DeliveryRover/Blueprints/Rover/BP_RoverPawn.bCanCharge` _asbp_rover_pawn)
                (if (`RoverPawn.IsCharging` _asbp_rover_pawn)
                  (set `local.HUD_InteractionPromptText` "E — остановить зарядку")
                  (set `local.HUD_HintText` "Идёт зарядка...")
                  (else
                    (set `local.HUD_InteractionPromptText` "E - зарядиться")
                    (set `local.HUD_HintText` "Зарядная станция рядом")))
                (set `local.HUD_bShowInteractionPrompt` true)
                (`/Game/DeliveryRover/Blueprints/UI/WBP_GameHUD.UpdateHUD` _gamehudref (`local.HUD_ObjectiveText`) (`local.HUD_OrderTitleText`) (`local.HUD_RouteText`) (`local.HUD_TimerText`) (`local.HUD_RewardText`) (`local.HUD_DistanceText`) (`local.HUD_BatteryText`) (`local.HUD_BatteryPercent`) (`local.HUD_CargoText`) (`local.HUD_CargoPercent`) (`local.HUD_CollisionsText`) (`local.HUD_HintText`) (`local.HUD_InteractionPromptText`) (`local.HUD_bShowInteractionPrompt`) :!label _label)))
            (:`Is Not Valid`
              (goto _label))))))))

(fn `UserConstructionScript`)