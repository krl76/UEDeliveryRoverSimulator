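; Player rover pawn for a delivery game, handling pause, phone app and interact input plus collision damage reporting.
; Pause opens a menu and pauses the game; the phone toggle swaps the HUD for the app, blocks rover input and changes input mode.
; Interact calls go to BP_OrderManager, as does damage from overlapping tagged obstacles and a forward sphere trace run every Tick, with debug drawing enabled.
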(event `self.OnPausePressed`
  (bind _returnvalue (`GameplayStatics.GetPlayerController` 0))
  ; OpenPause
  (`/Engine/EditorBlueprintResources/StandardMacros.IsValid` (`self.PauseMenuRef`)
    (:`Is Valid`
      (`KismetSystemLibrary.PrintString` "PauseIsValid"))
    (:`Is Not Valid`
      (`KismetSystemLibrary.PrintString` "PauseIsNotValid")
      (bind _returnvalue_2 (`|CreateWidget` "/Game/DeliveryRover/Blueprints/UI/WBP_PauseMenu.WBP_PauseMenu_C" _returnvalue))
      (bind _output_get (set `self.PauseMenuRef` _returnvalue_2))
      (`UserWidget.AddToViewport` _output_get 100)
      (`GameplayStatics.SetGamePaused` true)
      (set `PlayerController.bShowMouseCursor` true _returnvalue)
      (`WidgetBlueprintLibrary.SetInputMode_UIOnlyEx` _returnvalue _output_get))))

(event `self.OnPhoneTogglePressed`
  (`/Engine/EditorBlueprintResources/StandardMacros.IsValid` (`self.PhoneAppRef`)
    (:`Is Valid`
      (`self.ClosePhoneApp`))
    (:`Is Not Valid`
      (`self.OpenPhoneApp`))))

(event `self.OnInteractPressed`
  (bind _returnvalue (`GameplayStatics.GetActorOfClass` "/Game/DeliveryRover/Blueprints/Gameplay/BP_OrderManager.BP_OrderManager_C"))
  (`/Game/DeliveryRover/Blueprints/Gameplay/BP_OrderManager.TryInteract` _returnvalue)
  (`KismetSystemLibrary.PrintString` "Interact pressed"))

(event `self.ReceiveActorBeginOverlap`
  (params (OtherActor :type "Actor Object Reference"))
  (`KismetSystemLibrary.PrintString` "Print String \"Rover overlap\"")
  (if (`self.ActorHasTag` OtherActor "DamageObstacle")
    (bind _returnvalue (`GameplayStatics.GetActorOfClass` "/Game/DeliveryRover/Blueprints/Gameplay/BP_OrderManager.BP_OrderManager_C"))
    (`/Game/DeliveryRover/Blueprints/Gameplay/BP_OrderManager.RegisterCollisionDamage` _returnvalue 0.05)
    (`KismetSystemLibrary.PrintString` "Overlap!")))

(event `self.ReceiveTick`
  (params (DeltaSeconds :type "Float (single-precision)"))
  (`self.CheckWorldCollisionDamage`))

(fn `CheckWorldCollisionDamage`
  (bind _returnvalue (+ (`self.K2_GetActorLocation`) (0.0 0.0 25.0)))
  (bind (_outhit _returnvalue_2) (`KismetSystemLibrary.SphereTraceSingle` :`Start` _returnvalue :`End` (+ _returnvalue (* (`self.GetActorForwardVector`) (100.0 100.0 100.0))) :`Radius` 25.0 :`TraceChannel` "TraceTypeQuery1" :`bTraceComplex` true :`DrawDebugType` "ForDuration"))
  (if _returnvalue_2
    (bind _returnvalue_3 (`GameplayStatics.GetActorOfClass` "/Game/DeliveryRover/Blueprints/Gameplay/BP_OrderManager.BP_OrderManager_C"))
    (`/Game/DeliveryRover/Blueprints/Gameplay/BP_OrderManager.RegisterCollisionDamage` _returnvalue_3 0.05)))

(fn `ClosePhoneApp`
  (bind _returnvalue (`GameplayStatics.GetPlayerController` 0))
  (bind _phoneappref (`self.PhoneAppRef`))
  (`/Engine/EditorBlueprintResources/StandardMacros.IsValid` _phoneappref
    (:`Is Valid`
      (`Widget.RemoveFromParent` _phoneappref)
      (set `self.PhoneAppRef` null)
      (`self.SetRoverInputBlocked` false)
      (bind _asbp_delivery_player_controller (cast `/Game/DeliveryRover/Blueprints/Core/BP_DeliveryPlayerController` _returnvalue))
      (`Widget.SetVisibility` (`/Game/DeliveryRover/Blueprints/Core/BP_DeliveryPlayerController.GameHUDRef` _asbp_delivery_player_controller) "Visible")
      (set `PlayerController.bShowMouseCursor` false _returnvalue)
      (`WidgetBlueprintLibrary.SetInputMode_GameOnly` _returnvalue))))

(fn `OpenPhoneApp`
  (bind _returnvalue (`GameplayStatics.GetPlayerController` 0))
  (bind _returnvalue_2 (`|CreateWidget` "/Game/DeliveryRover/Blueprints/UI/WBP_PhoneApp.WBP_PhoneApp_C" _returnvalue))
  (bind _output_get (set `self.PhoneAppRef` _returnvalue_2))
  (`UserWidget.AddToViewport` _output_get 50)
  (`self.SetRoverInputBlocked` true)
  (bind _asbp_delivery_player_controller (cast `/Game/DeliveryRover/Blueprints/Core/BP_DeliveryPlayerController` _returnvalue))
  (`Widget.SetVisibility` (`/Game/DeliveryRover/Blueprints/Core/BP_DeliveryPlayerController.GameHUDRef` _asbp_delivery_player_controller) "Collapsed")
  (set `PlayerController.bShowMouseCursor` true _returnvalue)
  (`WidgetBlueprintLibrary.SetInputMode_GameAndUIEx` _returnvalue _output_get))

(fn `UserConstructionScript`)