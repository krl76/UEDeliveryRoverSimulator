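; Placeable narrow-leaf tree actor for Downtown West that pairs a static tree mesh with a falling-leaf Niagara effect.
; The construction script assigns the configured Niagara system, offsets the emitter by a location variable and pushes minimum and maximum lifetime and spawn rate into its float parameters.
; It also sets the tree mesh from a variable, so each instance can vary.
; The event graph holds no runtime logic.
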(fn `UserConstructionScript`
  (bind _ns_narrowleavesfalling (`self.NS_NarrowLeavesFalling`))
  (`NiagaraComponent.SetAsset` _ns_narrowleavesfalling (`self.Set Niagara Leaf System`))
  (`SceneComponent.K2_AddRelativeLocation` _ns_narrowleavesfalling (`self.Leaf Emitter Location`) false false)
  (`NiagaraComponent.SetVariableFloat` _ns_narrowleavesfalling "Lifetime_Minimum" (`self.Lifetime_Minimum`))
  (`NiagaraComponent.SetVariableFloat` _ns_narrowleavesfalling "Lifetime_Maximum" (`self.Lifetime Maximum`))
  (`NiagaraComponent.SetVariableFloat` _ns_narrowleavesfalling "SpawnRate_Maximum" (`self.Spawn Rate Maximum`))
  (`NiagaraComponent.SetVariableFloat` _ns_narrowleavesfalling "SpawnRate_Minimum" (`self.Spawn Rate Minimum`))
  (`StaticMeshComponent.SetStaticMesh` (`self.TreeMeshNarrow`) (`self.Tree Mesh`)))